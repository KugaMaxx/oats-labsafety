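; Chemical storage cabinet for an AR training task, completed by returning detached items and closing the door.
; Matching MSDS pages and vent are destroyed on overlap, revealing hidden built-in versions, while bottle overlaps adjust DetachedItemNum.
; Both bottle branches cast to Thinner, so it counts twice and Acetone never.
; A looping timer rotates the grabbed door from controller position; drops and count changes check for completion.
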(event `self.ReceiveBeginPlay`
  (`parent.ReceiveBeginPlay`)
  (`SceneComponent.SetHiddenInGame` (`self.Bottle Thinner`) true true)
  (`SceneComponent.SetHiddenInGame` (`self.Bottle Acetone`) true true)
  (`SceneComponent.SetHiddenInGame` (`self.MSDS Page Thinner`) true true)
  (`SceneComponent.SetHiddenInGame` (`self.MSDS Page Acetone`) true true)
  (`SceneComponent.SetHiddenInGame` (`self.Cabinet VentL`) true true))

(event `self.ReceiveTick`
  (params (DeltaSeconds :type "Float (single-precision)"))
  (`parent.ReceiveTick` DeltaSeconds))

(event `self.Grab Door.OnGrabbed`
  (`KismetSystemLibrary.K2_SetTimer` null "Rotate the Cabinet Door" 0.01 true))

(event `self.Grab Door.OnDropped`
  (`KismetSystemLibrary.K2_ClearTimer` null "Rotate the Cabinet Door")
  (`self.Check Tidy Status`))

(event `self.Box MSDS.OnComponentBeginOverlap`
  (params (OverlappedComponent :type "PrimitiveComponent Object Reference") (OtherActor :type "Actor Object Reference") (OtherComp :type "PrimitiveComponent Object Reference") (OtherBodyIndex :type Integer) (bFromSweep :type Boolean) (SweepResult :type "HitResult Structure (by ref)"))
  (bind _msds_page_thinner (`self.MSDS Page Thinner`))
  (bind _msds_page_acetone (`self.MSDS Page Acetone`))
  (`|ExecutionSequence`
    (:`then_0`
      (bind _asbp_detached_msds_page_thinner (cast `/Game/ARTraining/Blueprints/Cabinet/BP_Detached_MSDS_Page_Thinner` OtherActor))
      (`self.K2_DestroyActor` _asbp_detached_msds_page_thinner)
      (`SceneComponent.SetHiddenInGame` _msds_page_thinner false true)
      (`PrimitiveComponent.SetSimulatePhysics` _msds_page_thinner true))
    (:`then_1`
      (bind _asbp_detached_msds_page_acetone (cast `/Game/ARTraining/Blueprints/Cabinet/BP_Detached_MSDS_Page_Acetone` OtherActor))
      (`self.K2_DestroyActor` _asbp_detached_msds_page_acetone)
      (`SceneComponent.SetHiddenInGame` _msds_page_acetone false true)
      (`PrimitiveComponent.SetSimulatePhysics` _msds_page_acetone true)))
  (set `self.Detached Item Num` (- (`self.Detached Item Num`) 1) :!label _label)
  (`self.Check Tidy Status`))

(event `self.Box VentL.OnComponentBeginOverlap`
  (params (OverlappedComponent :type "PrimitiveComponent Object Reference") (OtherActor :type "Actor Object Reference") (OtherComp :type "PrimitiveComponent Object Reference") (OtherBodyIndex :type Integer) (bFromSweep :type Boolean) (SweepResult :type "HitResult Structure (by ref)"))
  (bind _asbp_detached_cabinet_vent (cast `/Game/ARTraining/Blueprints/Cabinet/BP_Detached_Cabinet_Vent` OtherActor))
  (`self.K2_DestroyActor` _asbp_detached_cabinet_vent)
  (`SceneComponent.SetHiddenInGame` (`self.Cabinet VentL`) false true)
  (goto _label))

(event `self.Box Cabinet.OnComponentBeginOverlap`
  (params (OverlappedComponent :type "PrimitiveComponent Object Reference") (OtherActor :type "Actor Object Reference") (OtherComp :type "PrimitiveComponent Object Reference") (OtherBodyIndex :type Integer) (bFromSweep :type Boolean) (SweepResult :type "HitResult Structure (by ref)"))
  (`|ExecutionSequence`
    (:`then_0`
      (cast `/Game/ARTraining/Blueprints/Cabinet/BP_Detached_Bottle_Thinner` OtherActor))
    (:`then_1`
      (cast `/Game/ARTraining/Blueprints/Cabinet/BP_Detached_Bottle_Thinner` OtherActor)))
  (set `self.Detached Item Num` (- (`self.Detached Item Num`) 1))
  (`self.Check Tidy Status`))

(event `self.Box Cabinet.OnComponentEndOverlap`
  (params (OverlappedComponent :type "PrimitiveComponent Object Reference") (OtherActor :type "Actor Object Reference") (OtherComp :type "PrimitiveComponent Object Reference") (OtherBodyIndex :type Integer))
  (`|ExecutionSequence`
    (:`then_0`
      (cast `/Game/ARTraining/Blueprints/Cabinet/BP_Detached_Bottle_Thinner` OtherActor))
    (:`then_1`
      (cast `/Game/ARTraining/Blueprints/Cabinet/BP_Detached_Bottle_Thinner` OtherActor)))
  (set `self.Detached Item Num` (+ (`self.Detached Item Num`) 1))
  (`self.Check Tidy Status`))

(event `Check Tidy Status`
  (bind (_relativerotation_roll _relativerotation_pitch _relativerotation_yaw) (`KismetMathLibrary.BreakRotator` (`SceneComponent.RelativeRotation` (`self.Cabinet Door`))))
  (if (<= (`self.Detached Item Num`) 0)
    (if (>= _relativerotation_yaw -1.0)
      (`self.Task Chemical Storage Complete`))))

(fn `Rotate the Cabinet Door`
  (bind _returnvalue_location (`KismetMathLibrary.BreakTransform` (`KismetMathLibrary.MakeRelativeTransform` (`SceneComponent.K2_GetComponentToWorld` (`/Game/VRTemplate/Blueprints/GrabComponent.MotionControllerRef` (`self.Grab Door`))) (`SceneComponent.K2_GetComponentToWorld` (`self.Scene Door`)))))
  (bind _returnvalue_x (`KismetMathLibrary.BreakVector` (- (`SceneComponent.RelativeLocation` (`self.Scene Door`)) _returnvalue_location)))
  (bind (_returnvalue_roll _returnvalue_pitch _returnvalue_yaw) (`KismetMathLibrary.BreakRotator` (`KismetMathLibrary.Quat_Rotator` (* (`KismetMathLibrary.Conv_RotatorToQuaternion` (`SceneComponent.RelativeRotation` (`self.Cabinet Door`))) (`KismetMathLibrary.Conv_RotatorToQuaternion` (`KismetMathLibrary.MakeRotator` 0.0 0.0 (* _returnvalue_x 1.0)))))))
  (`SceneComponent.K2_SetRelativeRotation` (`self.Cabinet Door`) (`KismetMathLibrary.MakeRotator` _returnvalue_roll _returnvalue_pitch (`KismetMathLibrary.FClamp` _returnvalue_yaw -120.0 0.0)) false false))

(fn `UserConstructionScript`
  (`parent.UserConstructionScript`))