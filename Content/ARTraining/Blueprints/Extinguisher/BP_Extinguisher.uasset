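; Grabbable fire extinguisher for motion-controller training, armed by dropping its pin and used to put out BP_Target_Fire.
; Grabbing the body disables its physics and enables input.
; Grabbing the hose sticks the hand mesh to it and starts a looping timer that rotates it after the controller, with clamped roll.
; Once armed, menu-toggle input spawns dry-powder Niagara and sphere-traces from the nozzle, lowering fire spawn rate until task completion fires.
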(event `self.ReceiveBeginPlay`
  (`parent.ReceiveBeginPlay`))

(event `self.Grab Body.OnGrabbed`
  (`PrimitiveComponent.SetSimulatePhysics` (`self.Extinguisher Body`) false)
  (set `/Game/VRTemplate/Blueprints/GrabComponent.Priority` 0 (`self.Grab Body`))
  (`self.EnableInput` (`GameplayStatics.GetPlayerController` 0)))

(event `self.Grab Hose.OnGrabbed`
  (`KismetSystemLibrary.K2_SetTimer` null "Rotate the Extinguisher Hose" 0.01 true)
  (for _array_element (`SceneComponent.GetChildrenComponents` (`/Game/VRTemplate/Blueprints/GrabComponent.MotionControllerRef` (`self.Grab Hose`)) false)
    (bind _asskeletal_mesh_component (cast `SkeletalMeshComponent` _array_element))
    (`/Engine/EditorBlueprintResources/StandardMacros.IsValid` _asskeletal_mesh_component
      (:`Is Valid`
        (bind _output_get (set `self.Sticky Hand` _asskeletal_mesh_component))
        (set `self.Sticky Hand Transform` (`SceneComponent.GetRelativeTransform` _output_get))
        (`SceneComponent.K2_AttachToComponent` (`self.Sticky Hand`) (`self.Grab Hose`) "None" "KeepWorld" "KeepWorld" "KeepWorld" true)))))

(event `self.Grab Body.OnDropped`
  (`PrimitiveComponent.SetSimulatePhysics` (`self.Extinguisher Body`) true)
  (set `/Game/VRTemplate/Blueprints/GrabComponent.Priority` 1 (`self.Grab Body`))
  (`self.DisableInput` (`GameplayStatics.GetPlayerController` 0)))

(event `self.Grab Hose.OnDropped`
  (`KismetSystemLibrary.K2_ClearTimer` null "Rotate the Extinguisher Hose")
  (`SceneComponent.K2_AttachToComponent` (`self.Sticky Hand`) (`/Game/VRTemplate/Blueprints/GrabComponent.MotionControllerRef` (`self.Grab Hose`)) "None" "KeepRelative" "KeepRelative" "KeepRelative" true)
  (`SceneComponent.K2_SetRelativeTransform` (`self.Sticky Hand`) (`self.Sticky Hand Transform`) false false))

(event `self.Grab Pin.OnDropped`
  (`PrimitiveComponent.SetSimulatePhysics` (`self.Extinguisher Pin`) true)
  (set `self.Is Activated` true))

(event `EnhancedInput|/Game/VRTemplate/Input/Actions/IA_Menu_Toggle_Right`
  (params (ActionValue :type Boolean) (ElapsedSeconds :type "Float (double-precision)") (TriggeredSeconds :type "Float (double-precision)") (InputAction :type "InputAction Object Reference" :default "/Game/VRTemplate/Input/Actions/IA_Menu_Toggle_Right.IA_Menu_Toggle_Right"))
  (bind (_returnvalue_location _returnvalue_rotation) (`KismetMathLibrary.BreakTransform` (`SceneComponent.K2_GetComponentToWorld` (`self.Extinguisher Nozzle`))))
  (bind (_returnvalue_location_2 _returnvalue_rotation_2) (`KismetMathLibrary.BreakTransform` (`SceneComponent.GetRelativeTransform` (`self.Extinguisher Nozzle`))))
  ;[0 0 0] Conducting Extinguishing
  (:`Triggered`
    (if (`self.Is Activated`) :!label _label
      (`|ExecutionSequence`
        (:`then_0`
          (`NiagaraFunctionLibrary.SpawnSystemAttached` "/Game/ARTraining/VFX/NS_DryPowder.NS_DryPowder" (`self.Extinguisher Hose`) "None" _returnvalue_location_2 _returnvalue_rotation_2 "KeepRelativeOffset"))
        (:`then_1`
          (bind (_outhit _returnvalue) (`KismetSystemLibrary.SphereTraceSingle` _returnvalue_location (+ _returnvalue_location (* (`KismetMathLibrary.GetUpVector` _returnvalue_rotation) (`KismetMathLibrary.Conv_DoubleToVector` 1000.0))) 20.0 "TraceTypeQuery1"))
          (if _returnvalue
            (bind _asbp_target_fire (cast `/Game/ARTraining/Blueprints/Extinguisher/BP_Target_Fire` (`.HitActor` (`GameplayStatics.BreakHitResult` _outhit))))
            (bind _returnvalue_2 (- (`/Game/ARTraining/Blueprints/Extinguisher/BP_Target_Fire.Spawn Rate` _asbp_target_fire) 1.0))
            (set `/Game/ARTraining/Blueprints/Extinguisher/BP_Target_Fire.Spawn Rate` _returnvalue_2 _asbp_target_fire)
            (`NiagaraComponent.SetVariableFloat` (`/Game/ARTraining/Blueprints/Extinguisher/BP_Target_Fire.NS_TurbulentFire` _asbp_target_fire) "SpawnRate" _returnvalue_2)
            (if (< _returnvalue_2 0.0)
              (`self.Task Fire Extinguishing Complete`))))))))

(event `EnhancedInput|/Game/VRTemplate/Input/Actions/IA_Menu_Toggle_Left`
  (params (ActionValue :type Boolean) (ElapsedSeconds :type "Float (double-precision)") (TriggeredSeconds :type "Float (double-precision)") (InputAction :type "InputAction Object Reference" :default "/Game/VRTemplate/Input/Actions/IA_Menu_Toggle_Left.IA_Menu_Toggle_Left"))
  ;[0 0 0] Conducting Extinguishing
  (:`Triggered`
    (goto _label)))

(fn `Rotate the Extinguisher Hose`
  (bind _returnvalue_location (`KismetMathLibrary.BreakTransform` (`KismetMathLibrary.MakeRelativeTransform` (`SceneComponent.K2_GetComponentToWorld` (`/Game/VRTemplate/Blueprints/GrabComponent.MotionControllerRef` (`self.Grab Hose`))) (`SceneComponent.K2_GetComponentToWorld` (`self.Scene Hose`)))))
  (bind (_returnvalue_x _returnvalue_y) (`KismetMathLibrary.BreakVector` (- (`SceneComponent.RelativeLocation` (`self.Scene Hose`)) _returnvalue_location)))
  (bind (_returnvalue_roll _returnvalue_pitch _returnvalue_yaw) (`KismetMathLibrary.BreakRotator` (`KismetMathLibrary.Quat_Rotator` (* (`KismetMathLibrary.Conv_RotatorToQuaternion` (`SceneComponent.RelativeRotation` (`self.Extinguisher Hose`))) (`KismetMathLibrary.Conv_RotatorToQuaternion` (`KismetMathLibrary.MakeRotator` (* _returnvalue_y 1.0)))))))
  (`SceneComponent.K2_SetRelativeRotation` (`self.Extinguisher Hose`) (`KismetMathLibrary.MakeRotator` (`KismetMathLibrary.FClamp` _returnvalue_roll -150.0 0.0) _returnvalue_pitch _returnvalue_yaw) false false))

(fn `UserConstructionScript`
  (`parent.UserConstructionScript`))