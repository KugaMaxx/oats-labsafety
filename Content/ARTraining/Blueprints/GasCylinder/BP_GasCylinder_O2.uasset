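; Oxygen gas cylinder for a training task, assembled and operated with motion-controller hands.
; Overlapping detached regulator and arrestor actors destroys them and reveals the built-in parts in order, completing the cylinder task.
; Aligned hands stick to valve or knob while looping timers turn controller rotation into clamped part rotation.
; The valve toggles gas via timelines driving both gauge needles; the knob moves the left needle, with grab types alternating between them.
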(event `self.ReceiveBeginPlay`
  (`parent.ReceiveBeginPlay`)
  (`SceneComponent.SetHiddenInGame` (`self.Regulator Body`) true true)
  (`SceneComponent.SetHiddenInGame` (`self.Flashback Arrestor`) true true))

(event `self.ReceiveTick`
  (params (DeltaSeconds :type "Float (single-precision)"))
  (`parent.ReceiveTick` DeltaSeconds))

(event `self.Box Mount.OnComponentBeginOverlap`
  (params (OverlappedComponent :type "PrimitiveComponent Object Reference") (OtherActor :type "Actor Object Reference") (OtherComp :type "PrimitiveComponent Object Reference") (OtherBodyIndex :type Integer) (bFromSweep :type Boolean) (SweepResult :type "HitResult Structure (by ref)"))
  ;[0 0 0] Installation
  (bind _asbp_detached_regulator (cast `/Game/ARTraining/Blueprints/GasCylinder/BP_Detached_Regulator` OtherActor))
  (`self.K2_DestroyActor` _asbp_detached_regulator)
  (`SceneComponent.SetHiddenInGame` (`self.Regulator Body`) false true))

(event `self.Box Regulator.OnComponentBeginOverlap`
  (params (OverlappedComponent :type "PrimitiveComponent Object Reference") (OtherActor :type "Actor Object Reference") (OtherComp :type "PrimitiveComponent Object Reference") (OtherBodyIndex :type Integer) (bFromSweep :type Boolean) (SweepResult :type "HitResult Structure (by ref)"))
  ;[0 0 0] Installation
  (if (not (`SceneComponent.bHiddenInGame` (`self.Regulator Body`)))
    (bind _asbp_detached_arrestor (cast `/Game/ARTraining/Blueprints/GasCylinder/BP_Detached_Arrestor` OtherActor))
    (`self.K2_DestroyActor` _asbp_detached_arrestor)
    (`SceneComponent.SetHiddenInGame` (`self.Flashback Arrestor`) false true)
    (set `self.Is Integrated` true)
    (`self.Task Gas Cylinder Complete`)))

(event `self.Grab Knob.OnGrabbed`
  ;[0 0 0] Regulator Knob
  (bind _is_sticked (`self.Stick Hand to Component` (`self.Grab Knob`) (`self.Scene Knob`)))
  (if _is_sticked
    (`KismetSystemLibrary.K2_SetTimer` null "Rotate the Regulator Knob" 0.01 true)))

(event `self.Grab Knob.OnDropped`
  (bind _relativerotation_roll (`KismetMathLibrary.BreakRotator` (`SceneComponent.RelativeRotation` (`self.Regulator PointerL`))))
  (bind _returnvalue (< _relativerotation_roll -5.0))
  ;[0 0 0] Regulator Knob
  (`self.Release Hand From Component` (`self.Grab Knob`))
  (`KismetSystemLibrary.K2_ClearTimer` null "Rotate the Regulator Knob")
  (if (`self.Is Turned On`)
    (if _returnvalue
      (`self.Task Pressure Regulation Complete (Turn On)`)
      (set `/Game/VRTemplate/Blueprints/GrabComponent.GrabType` "NewEnumerator3" (`self.Grab Valve`))
      (set `/Game/VRTemplate/Blueprints/GrabComponent.GrabType` "NewEnumerator0" (`self.Grab Knob`)))
    (elif (not _returnvalue)
      (`self.Task Pressure Regulation Complete (Turn Off)`)
      (set `/Game/VRTemplate/Blueprints/GrabComponent.GrabType` "NewEnumerator3" (`self.Grab Valve`))
      (set `/Game/VRTemplate/Blueprints/GrabComponent.GrabType` "NewEnumerator0" (`self.Grab Knob`)))))

(event `Update Left Pointer`
  ;[0 0 0] Regulator Knob
  (if (`self.Is Turned On`)
    (`SceneComponent.K2_SetRelativeRotation` (`self.Regulator PointerL`) (`KismetMathLibrary.MakeRotator` (* (`self.Relief Degree`) -1.0)) false false)))

(event `self.Grab Valve.OnGrabbed`
  ;[0 0 0] Main Valve
  (bind _is_sticked (`self.Stick Hand to Component` (`self.Grab Valve`) (`self.Scene Valve`)))
  (if _is_sticked
    (set `self.Is Before On` (`self.Is Turned On`))
    (`KismetSystemLibrary.K2_SetTimer` null "Rotate the GasCylinder Valve" 0.01 true)))

(event `self.Grab Valve.OnDropped`
  ;[0 0 0] Main Valve
  (`self.Release Hand From Component` (`self.Grab Valve`))
  (`KismetSystemLibrary.K2_ClearTimer` null "Rotate the GasCylinder Valve")
  (if (not (== (`self.Is Before On`) (`self.Is Turned On`)))
    (set `/Game/VRTemplate/Blueprints/GrabComponent.GrabType` "NewEnumerator0" (`self.Grab Valve`))
    (set `/Game/VRTemplate/Blueprints/GrabComponent.GrabType` "NewEnumerator3" (`self.Grab Knob`))))

(event `Update Right Pointer`
  ;[0 0 0] Main Valve
  (if (`self.Is Turned On`)
    (if (< (`self.Main Degree`) (* (`self.Threshold`) 0.8))
      (bind (_direction _degree) (`Timeline|Turn Off Timeline` :!via `PlayFromStart`)
        (:`Update`
          (`SceneComponent.K2_SetRelativeRotation` (`self.Regulator PointerR`) (`KismetMathLibrary.MakeRotator` (* (`self.Threshold`) _degree)) false false)
          (set `self.Is Turned On` false)
          (`SceneComponent.K2_SetRelativeRotation` (`self.Regulator PointerL`) (`KismetMathLibrary.MakeRotator` (* (`self.Relief Degree`) _degree)) false false))))
    (elif (> (`self.Main Degree`) (* (`self.Threshold`) 1.2))
      (bind (_direction_2 _degree_2) (`Timeline|Turn On Timeline` :!via `PlayFromStart`)
        (:`Update`
          (`SceneComponent.K2_SetRelativeRotation` (`self.Regulator PointerR`) (`KismetMathLibrary.MakeRotator` (* (`self.Threshold`) _degree_2)) false false)
          (set `self.Is Turned On` true)
          (`SceneComponent.K2_SetRelativeRotation` (`self.Regulator PointerL`) (`KismetMathLibrary.MakeRotator` (* (`self.Relief Degree`) _degree_2)) false false))))))

(fn `Release Hand From Component`
  (params (`Grab Component` :type "/Game/VRTemplate/Blueprints/GrabComponent Object Reference"))
  (`SceneComponent.K2_AttachToComponent` (`self.Sticky Hand`) (`/Game/VRTemplate/Blueprints/GrabComponent.MotionControllerRef` (`local.Grab Component`)) "None" "KeepRelative" "KeepRelative" "KeepRelative" true)
  (`SceneComponent.K2_SetRelativeTransform` (`self.Sticky Hand`) (`self.Sticky Hand Transform`) false false))

(fn `Rotate the GasCylinder Valve`
  (bind _returnvalue (* (`KismetMathLibrary.SelectFloat` 1.0 -1.0 (`|EnumEquality` (`/Game/VRTemplate/Blueprints/GrabComponent.GetHeldByHand` (`self.Grab Valve`)) "Left")) (.pitch (.rotation (`KismetMathLibrary.MakeRelativeTransform` (`SceneComponent.K2_GetComponentToWorld` (`/Game/VRTemplate/Blueprints/GrabComponent.MotionControllerRef` (`self.Grab Valve`))) (`SceneComponent.K2_GetComponentToWorld` (`self.Scene Valve`)))))))
  (bind _returnvalue_2 (+ (`self.Main Degree`) (* 1.0 _returnvalue)))
  (if (`KismetMathLibrary.InRange_FloatFloat` _returnvalue_2 0.0 120.0)
    (bind _output_get (set `self.Main Degree` _returnvalue_2))
    (if (`KismetMathLibrary.InRange_FloatFloat` _output_get -120.0 120.0)
      (`SceneComponent.K2_SetRelativeRotation` (`self.GasCylinder Valve`) (`KismetMathLibrary.Quat_Rotator` (* (`KismetMathLibrary.Conv_RotatorToQuaternion` (`SceneComponent.RelativeRotation` (`self.GasCylinder Valve`))) (`KismetMathLibrary.Conv_RotatorToQuaternion` (`KismetMathLibrary.MakeRotator` 0.0 0.0 _returnvalue)))) false false)
      (`self.Update Right Pointer`))))

(fn `Rotate the Regulator Knob`
  (bind _returnvalue (* (`KismetMathLibrary.SelectFloat` 1.0 -1.0 (`|EnumEquality` (`/Game/VRTemplate/Blueprints/GrabComponent.GetHeldByHand` (`self.Grab Knob`)) "Right")) (.pitch (.rotation (`KismetMathLibrary.MakeRelativeTransform` (`SceneComponent.K2_GetComponentToWorld` (`/Game/VRTemplate/Blueprints/GrabComponent.MotionControllerRef` (`self.Grab Knob`))) (`SceneComponent.K2_GetComponentToWorld` (`self.Scene Knob`)))))))
  (bind _returnvalue_2 (+ (`self.Relief Degree`) (* -1.0 _returnvalue)))
  (if (`KismetMathLibrary.InRange_FloatFloat` _returnvalue_2 0.0 120.0)
    (bind _output_get (set `self.Relief Degree` _returnvalue_2))
    (if (`KismetMathLibrary.InRange_FloatFloat` _output_get -120.0 120.0)
      (`SceneComponent.K2_SetRelativeRotation` (`self.Regulator Knob`) (`KismetMathLibrary.Quat_Rotator` (* (`KismetMathLibrary.Conv_RotatorToQuaternion` (`SceneComponent.RelativeRotation` (`self.Regulator Knob`))) (`KismetMathLibrary.Conv_RotatorToQuaternion` (`KismetMathLibrary.MakeRotator` _returnvalue)))) false false)
      (`self.Update Left Pointer`))))

(fn `Stick Hand to Component`
  (params (`Grab Component` :type "/Game/VRTemplate/Blueprints/GrabComponent Object Reference") (`Scene Component` :type "SceneComponent Object Reference"))
  (returns (`Is Sticked` :type Boolean))
  (`|ExecutionSequence`
    (:`then_0`
      (for _array_element (`SceneComponent.GetChildrenComponents` (`/Game/VRTemplate/Blueprints/GrabComponent.MotionControllerRef` (`local.Grab Component`)) false)
        (bind _asskeletal_mesh_component (cast `SkeletalMeshComponent` _array_element))
        (`/Engine/EditorBlueprintResources/StandardMacros.IsValid` _asskeletal_mesh_component
          (:`Is Valid`
            (bind _output_get (set `self.Sticky Hand` _asskeletal_mesh_component))
            (set `self.Sticky Hand Transform` (`SceneComponent.GetRelativeTransform` _output_get))))))
    (:`then_1`
      (if (>= (`KismetMathLibrary.Dot_VectorVector` (`SceneComponent.GetUpVector` (`self.Sticky Hand`)) (`SceneComponent.GetUpVector` (`local.Grab Component`))) 0.95)
        (`SceneComponent.K2_SetWorldRotation` (`local.Scene Component`) (`SceneComponent.K2_GetComponentRotation` (`/Game/VRTemplate/Blueprints/GrabComponent.MotionControllerRef` (`local.Grab Component`))) false false)
        (`SceneComponent.K2_AttachToComponent` (`self.Sticky Hand`) (`local.Scene Component`) "None" "KeepWorld" "KeepWorld" "KeepWorld" true)
        (return true)
        (else
          (return false))))))

(fn `UserConstructionScript`
  (`parent.UserConstructionScript`))