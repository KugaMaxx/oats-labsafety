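; BP_GasHose is a gas hose for the AR training project, with two ring ends that snap onto matching fittings.
; Box overlaps check for the Type I ring on BP_Reactor and the Type L ring on BP_GasCylinder_O2.
; On a match, that end's grab type changes, and its ring attaches to the fitting and takes its world transform.
; Only the cylinder connection also sets the cylinder's IsLinked flag.
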(event `self.Box TypeI.OnComponentBeginOverlap`
  (params (OverlappedComponent :type "PrimitiveComponent Object Reference") (OtherActor :type "Actor Object Reference") (OtherComp :type "PrimitiveComponent Object Reference") (OtherBodyIndex :type Integer) (bFromSweep :type Boolean) (SweepResult :type "HitResult Structure (by ref)"))
  (bind _asbp_reactor (cast `/Game/ARTraining/Blueprints/Reactor/BP_Reactor` OtherActor))
  (if (== (`/Game/ARTraining/Blueprints/Reactor/BP_Reactor.GasRing TypeI` _asbp_reactor) OtherComp)
    (set `/Game/VRTemplate/Blueprints/GrabComponent.GrabType` "NewEnumerator0" (`self.Grab TypeI`))
    (`SceneComponent.K2_AttachToComponent` (`self.GasRing TypeI`) OtherComp "None" "KeepWorld" "KeepWorld" "KeepWorld" true)
    (`SceneComponent.K2_SetWorldTransform` (`self.GasRing TypeI`) (`SceneComponent.K2_GetComponentToWorld` OtherComp) false false)))

(event `self.Box TypeL.OnComponentBeginOverlap`
  (params (OverlappedComponent :type "PrimitiveComponent Object Reference") (OtherActor :type "Actor Object Reference") (OtherComp :type "PrimitiveComponent Object Reference") (OtherBodyIndex :type Integer) (bFromSweep :type Boolean) (SweepResult :type "HitResult Structure (by ref)"))
  (bind _asbp_gas_cylinder_o2 (cast `/Game/ARTraining/Blueprints/GasCylinder/BP_GasCylinder_O2` OtherActor))
  (if (== (`/Game/ARTraining/Blueprints/GasCylinder/BP_GasCylinder_O2.GasRing TypeL` _asbp_gas_cylinder_o2) OtherComp)
    (set `/Game/ARTraining/Blueprints/GasCylinder/BP_GasCylinder_O2.Is Linked` true _asbp_gas_cylinder_o2)
    (set `/Game/VRTemplate/Blueprints/GrabComponent.GrabType` "NewEnumerator0" (`self.Grab TypeL`))
    (`SceneComponent.K2_AttachToComponent` (`self.GasRing TypeL`) OtherComp "None" "KeepWorld" "KeepWorld" "KeepWorld" true)
    (`SceneComponent.K2_SetWorldTransform` (`self.GasRing TypeL`) (`SceneComponent.K2_GetComponentToWorld` OtherComp) false false)))

(fn `UserConstructionScript`)